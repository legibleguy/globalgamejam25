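; Moving obstacle that destroys the player character on overlap and chains the spawning of further obstacles.
; Tick moves it along Y at a speed scaled by input and wind, tracking distance travelled.
; Past a random fraction of its starting distance to the player, it spawns one successor at its original location.
; The successor's mesh comes from shuffled data table rows with per-row probability rolls, applied in the construction script.
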(event `self.ReceiveBeginPlay`
  (`|ExecutionSequence`
    (:`then_0`
      (bind _outactors (`GameplayStatics.GetAllActorsOfClass` "/Game/Developers/Andy/Player/BP_PlayerCharacter.BP_PlayerCharacter_C"))
      (bind _output (`|GetArrayItem` _outactors))
      (`/Engine/EditorBlueprintResources/StandardMacros.IsValid` _output
        (:`Is Valid`
          (set `self.PlayerRef` _output))))
    (:`then_1`
      (`self.PlayerRef`
        (:`then`
          (set `self.ObstacleSpawnLocation` (`self.K2_GetActorLocation`))
          (bind _output_get (set `self.TotalDistance ToActor` (`self.GetDistanceTo` (`GameplayStatics.GetPlayerPawn` 0) self)))
          (set `self.DistanceToTriggerSpawn` (* _output_get (`KismetMathLibrary.RandomFloatInRange` 0.1 0.9))))
        (:`else`)))))

(event `self.ReceiveActorBeginOverlap`
  (params (OtherActor :type "Actor Object Reference"))
  (if (== OtherActor (`self.PlayerRef`))
    (`self.K2_DestroyActor` (`self.PlayerRef`))))

(event `self.ReceiveTick`
  (params (DeltaSeconds :type "Float (single-precision)"))
  (bind _returnvalue (* DeltaSeconds (`self.Speed`) (`/Game/Developers/Andy/Player/Lib_Player.Get Speed from Input and Wind` self)))
  (bind _output_get (set `self.TotalDistanceTravelled` (+ (stale _output_get) (`KismetMathLibrary.Abs` _returnvalue))))
  (`self.K2_SetActorLocation` (+ (`self.K2_GetActorLocation`) (`KismetMathLibrary.MakeVector` 0.0 _returnvalue)))
  (`self.NewSpawnedObstacle`
    (:`then`)
    (:`else`
      (if (> (`self.TotalDistanceTravelled`) (`self.DistanceToTriggerSpawn`))
        (bind _returnvalue_2 (`|SpawnActorFromClass` "BP_Obstacle_C" (`KismetMathLibrary.Conv_VectorToTransform` (`self.ObstacleSpawnLocation`)) "AlwaysSpawn" "MultiplyWithRoot" null (`self.PickNewObstacleMesh`) null))
        (set `self.NewSpawnedObstacle` _returnvalue_2)))))

(fn `PickNewObstacleMesh`
  (returns (ObstacleMesh :type "StaticMesh Object Reference"))
  (locals (Names :type "Array of Name"))
  (bind _outrownames (`DataTableFunctionLibrary.GetDataTableRowNames` "/Game/Obstacles/DT_ObstaclesToSpawn.DT_ObstaclesToSpawn"))
  (bind _output_get (set `local.Names` _outrownames))
  (`KismetArrayLibrary.Array_Shuffle` _output_get)
  (for _array_element _output_get
    (bind _returnvalue (`|GetDataTableRow` "/Game/Obstacles/DT_ObstaclesToSpawn.DT_ObstaclesToSpawn" _array_element)
      (:`then`
        (bind (_obstaclemesh _probabilitytospawn) (break `/Game/Obstacles/Struct_ObstacleData` _returnvalue))
        (if (`KismetMathLibrary.RandomBoolWithWeight` _probabilitytospawn)
          (return _obstaclemesh))))))

(fn `UserConstructionScript`
  (bind _initialmesh (`self.InitialMesh`)
    (:`then`
      (`StaticMeshComponent.SetStaticMesh` (`self.StaticMesh`) _initialmesh))
    (:`else`)))